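; Static helper functions for VR hand-tracked spellcasting, working on arrays of hand joint transforms.
; Pose helpers test joint proximity and use dot products to classify finger curl against the palm and palm facing relative to the camera.
; Spell helpers detect ending postures and map two-step element-plus-posture feeds to spell names.
; A palm-forward sphere trace finds a mostly upward-facing surface and returns a transform there with the hand's yaw.
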(fn AreJointsTouching
  (params (Joint%20Transforms :type Array%20of%20Transforms) (Joint%201 :type EHandKeypoint%20Enum :default "Palm") (Joint%202 :type EHandKeypoint%20Enum :default "Palm") (Threshold :type Integer))
  (return (<= (Math|Vector|Distance(Vector) (.location (Utilities|Array|Get(acopy) Joint%20Transforms (Class|HandKeypointConversion|ToInt32(HandKeypoint) Joint%201))) (.location (Utilities|Array|Get(acopy) Joint%20Transforms (Class|HandKeypointConversion|ToInt32(HandKeypoint) Joint%202)))) Threshold)))

(fn GetFingerCurl
  (params (Joint%20Transforms :type Array%20of%20Transforms) (Proximal :type EHandKeypoint%20Enum :default "Palm") (Intermediate :type EHandKeypoint%20Enum :default "Palm") (Distal :type EHandKeypoint%20Enum :default "Palm") (Tip :type EHandKeypoint%20Enum :default "Palm"))
  (bind _returnvalue (Class|HandKeypointConversion|ToInt32(HandKeypoint) Tip))
  (bind _returnvalue_2 (Utilities|Enum|LiteralenumEHandKeypoint "Palm"))
  (bind _returnvalue_3 (Class|HandKeypointConversion|ToInt32(HandKeypoint) _returnvalue_2))
  (bind _output (Utilities|Array|Get(acopy) Joint%20Transforms _returnvalue))
  (bind _z (Math|Rotator|GetAxes (.rotation _output)))
  (bind _output_2 (Utilities|Array|Get(acopy) Joint%20Transforms _returnvalue_3))
  (bind _returnvalue_4 (Math|Vector|Normalize _z))
  (bind _z_2 (Math|Rotator|GetAxes (.rotation _output_2)))
  (bind _returnvalue_5 (Math|Vector|Normalize _z_2))
  (bind _returnvalue_6 (Math|Vector|DotProduct _returnvalue_4 _returnvalue_5))
  (if (Math|Float|InRange(Float) _returnvalue_6 -1.0 -0.707)
    (return 2)
    (elif (Math|Float|InRange(Float) _returnvalue_6 -0.707 0.707)
      (return 1)
      (elif (Math|Float|InRange(Float) _returnvalue_6 0.0 0.707)
        (return 0)))))

(fn GetPalmFacing
  (params (Joint%20Transforms :type Array%20of%20Transforms))
  (bind _returnvalue (Game|GetPlayerCameraManager 0))
  (bind _returnvalue_2 (Utilities|Enum|LiteralenumEHandKeypoint "Palm"))
  (bind _returnvalue_3 (Transformation|GetActorRotation _returnvalue))
  (bind _returnvalue_4 (Class|HandKeypointConversion|ToInt32(HandKeypoint) _returnvalue_2))
  (bind _returnvalue_5 (Math|Vector|GetRightVector _returnvalue_3))
  (bind _returnvalue_6 (Math|Vector|GetUpVector _returnvalue_3))
  (bind _output (Utilities|Array|Get(acopy) Joint%20Transforms _returnvalue_4))
  (bind _returnvalue_7 (Math|Vector|GetForwardVector (.rotation _output)))
  (bind _returnvalue_8 (Math|Vector|Normalize _returnvalue_5))
  (bind _returnvalue_9 (Math|Vector|Normalize _returnvalue_6))
  (bind _returnvalue_10 (Math|Vector|Normalize _returnvalue_7))
  (bind _returnvalue_11 (Math|Vector|DotProduct _returnvalue_10 _returnvalue_8))
  (bind _returnvalue_12 (Math|Vector|DotProduct _returnvalue_10 _returnvalue_9))
  (if (Math|Float|InRange(Float) (Math|Vector|DotProduct _returnvalue_10 (Math|Vector|Normalize (Math|Vector|GetForwardVector _returnvalue_3))) 0.707 1.0)
    ;[0.15 0.15 0.15 0.5] 0: Forward
    (return 0)
    (elif (Math|Float|InRange(Float) _returnvalue_11 0.707 1.0)
      ;[0.15 0.15 0.15 0.5] 3: Right
      (return 3)
      (elif (Math|Float|InRange(Float) _returnvalue_11 -1.0 -0.707)
        ;[0.15 0.15 0.15 0.5] 2: Left
        (return 2)
        (elif (Math|Float|InRange(Float) _returnvalue_12 0.707 1.0)
          ;[0.15 0.15 0.15 0.5] 1: Up
          (return 1)
          (elif (Math|Float|InRange(Float) _returnvalue_12 -1.0 -0.5)
            ;[0.15 0.15 0.15 0.5] 4: Down
            (return 4)))))))

(fn IsValidSpellEnd
  (params (Posture :type Name))
  (return (or (== Posture "Projectile") (== Posture "Special"))))

(fn ParseSpell
  (params (Spell%20Feed :type Array%20of%20Names))
  (bind _output (Utilities|Array|Get(acopy) Spell%20Feed 1))
  (bind _output_2 (Utilities|Array|Get(acopy) Spell%20Feed))
  ;[0.15 0.15 0.15 0.5] Length of 2
  (if (== (Utilities|Array|Length Spell%20Feed) 2)
    ;[0.15 0.15 0.15 0.5] Fire Bolt
    (if (and (== _output_2 "Fire") (== _output "Projectile"))
      (return "Fire Bolt")
      (else
        ;[0.15 0.15 0.15 0.5] Ice Bolt
        (if (and (== _output_2 "Water") (== _output "Projectile"))
          (return "Ice Bolt")
          (else
            ;[0.15 0.15 0.15 0.5] Air Bolt
            (if (and (== _output_2 "Air") (== _output "Projectile"))
              (return "Air Bolt")
              (else
                ;[0.15 0.15 0.15 0.5] Earth Bolt
                (if (and (== _output_2 "Earth") (== _output "Projectile"))
                  (return "Earth Bolt")
                  (else
                    ;[0.15 0.15 0.15 0.5] Earth Pillar
                    (if (and (== _output_2 "Earth") (== _output "Special"))
                      (return "Earth Pillar")
                      (else
                        ;[0.15 0.15 0.15 0.5] Scorch
                        (if (and (== _output_2 "Fire") (== _output "Special"))
                          (return "Scorch"))))))))))))
    (else
      (return "None"))))

(fn ComputeRaycastLocation
  (params (Spawn%20Transform :type Array%20of%20Transforms))
  (bind _returnvalue (Utilities|Enum|LiteralenumEHandKeypoint "Palm"))
  (bind _returnvalue_2 (Class|HandKeypointConversion|ToInt32(HandKeypoint) _returnvalue))
  (bind _output (Utilities|Array|Get(acopy) Spawn%20Transform _returnvalue_2))
  (bind _returnvalue_3 (Math|Vector|GetForwardVector (.rotation _output)))
  (bind _array (Utilities|Array|MakeArray (.location _output)))
  (bind _returnvalue_4 (Math|Conversions|RotationFromXVector _returnvalue_3))
  (bind _output_2 (Utilities|Array|Get(acopy) _array))
  (bind _array_2 (Utilities|Array|MakeArray _returnvalue_4))
  (bind _outhits (Collision|MultiSphereTraceByChannel 0 _output_2 (+ _output_2 (* (Math|Vector|GetForwardVector (Class|KismetMathLibrary|QuatRotator (* (* (Math|Conversions|ToQuaternion(Rotator) (Utilities|Array|Get(acopy) _array_2)) (Math|Conversions|ToQuaternion(Rotator) (Math|Rotator|MakeRotator 0.0 0.0 0.0))) (Math|Conversions|ToQuaternion(Rotator) (Math|Rotator|MakeRotator 0.0 0.0 0.0))))) 1.5e+03)) 0.0 "TraceTypeQuery1" false 0 "ForDuration"))
  (for _array_element _outhits
    (if (> (Math|Vector|DotProduct (.ImpactNormal (Collision|BreakHitResult _array_element)) "0.000000,0.000000,1.000000") 0.5)
      (return (Math|Transform|MakeTransform (.Location (Collision|BreakHitResult _array_element)) (Math|Rotator|MakeRotator 0.0 0.0 (+ (.Yaw (Math|Rotator|BreakRotator (Utilities|Array|Get(acopy) _array_2))) 0.0)))))))