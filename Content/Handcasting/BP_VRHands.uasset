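; VR hand-tracking spellcaster that draws both hands as instanced-mesh joints and turns right-hand gesture chains into spells.
; A wolf pose starts a chain, and a looping timer samples postures into SpellFeed: flat-palm orientation gives an element, gun or claw gives a shape.
; Hand material shows each posture.
; A valid end posture stops sampling, then a polling timer triggers parsing and casts palm-directed bolts or raycast-placed Earth Pillar and Scorch.
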(event Custom|Hold%20Posture
  (bind _transforms (CallFunction|GetJointTransforms "Right"))
  (bind _isvalidjointtransform (CallFunction|IsJointTransformValid _transforms))
  (if _isvalidjointtransform
    (Variables|Default|SetCurrent%20Posture "None")
    (bind _posture (CallFunction|ReadPosture _transforms))
    (Variables|Default|SetCurrent%20Posture _posture)
    (bind _posture_2 (CallFunction|ReadPosture _transforms))
    (Utilities|Array|Add (Variables|Default|GetSpell%20Feed) _posture_2)
    (bind _valid_end_posture_ (CallFunction|IsValidSpellEnd _posture_2))
    (if _valid_end_posture_
      (Variables|Default|SetisCasting false)
      (Utilities|Time|ClearandInvalidateTimerbyHandle (stale EventTick _returnvalue)))))

(event Custom|Check%20Casting%20End
  ;[0.15 0.15 0.15 0.5] After loop: verify spell chain and then cast
  (if (not (Variables|Default|GetisCasting))
    (Utilities|FlowControl|Sequence
      (:then_0
        (Utilities|Time|ClearandInvalidateTimerbyHandle (stale EventTick _returnvalue_2)))
      (:then_1
        (Utilities|FlowControl|Delay 0.6)
        (bind _spell (CallFunction|ParseSpell (Variables|Default|GetSpell%20Feed)))
        (CallFunction|CastSpell (stale EventTick _transforms_2) _spell)
        (Utilities|FlowControl|Delay 0.15)
        (CallFunction|ChangeHandMaterial "/Game/Handcasting/Materials/HandCubes.HandCubes")))))

(event Custom|Add%20Posture
  (bind _transforms (CallFunction|GetJointTransforms "Right"))
  (bind _isvalidjointtransform (CallFunction|IsJointTransformValid _transforms))
  (if _isvalidjointtransform
    (bind _posture (CallFunction|ReadPosture _transforms))
    (Development|PrintString (Utilities|String|ToString(Name) _posture))
    (Utilities|Array|Add (Variables|Default|GetSpell%20Feed) _posture)))

(event EventBeginPlay)

(event Collision|EventActorBeginOverlap
  (params (OtherActor :type Actor%20Object%20Reference)))

(event EventTick
  (params (DeltaSeconds :type Float%20%28single-precision%29))
  (CallFunction|ClearHands)
  (Utilities|FlowControl|Sequence
    (:then_0
      (bind _transforms (CallFunction|GetJointTransforms "Left"))
      (CallFunction|DrawHand _transforms))
    (:then_1
      (bind _transforms_2 (CallFunction|GetJointTransforms "Right"))
      (CallFunction|DrawHand _transforms_2)
      (bind _isvalidjointtransform (CallFunction|IsJointTransformValid _transforms_2))
      (if _isvalidjointtransform
        ;[0.15 0.15 0.15 0.5] Check if we are starting or ending a spell chain
        (bind _posture_met (CallFunction|Handpose:Wolf _transforms_2))
        (if (and _posture_met (not (Variables|Default|GetisCasting)))
          (Variables|Default|SetisCasting true)
          (CallFunction|ChangeHandMaterial "/Game/Handcasting/Materials/HandCubes_Casting.HandCubes_Casting")
          (Utilities|Array|Clear (Variables|Default|GetSpell%20Feed))
          ;[0.15 0.15 0.15 0.5] Loop body: transcribe spell postures
          (bind _returnvalue (Utilities|Time|SetTimerbyEvent (delegate Custom|Hold%20Posture) 1.0 true))
          (bind _returnvalue_2 (Utilities|Time|SetTimerbyEvent (delegate Custom|Check%20Casting%20End) 0.1 true)))))))

(fn ConstructionScript)

(fn GetJointTransforms
  (params (Hand :type EControllerHand%20Enum :default "Left"))
  ;[0 0 0 0.5] Get hand tracking data
  (bind _handtrackingstate (Class|HeadMountedDisplayFunctionLibrary|GetHandTrackingState 0 "UnrealWorldSpace" Hand))
  ;[0.15 0.15 0.15 0.5] If the controller for this hand is active, we ignore the hand tracking data
  (bind _motioncontrollerstate (Class|HeadMountedDisplayFunctionLibrary|GetMotionControllerState 0 "UnrealWorldSpace" Hand "Aim"))
  (if (and (not (.bvalid _motioncontrollerstate)) (.bValid (Utilities|Struct|BreakXRHandTrackingState _handtrackingstate)))
    ;[0.15 0.15 0.15 0.5] validate the hand tracking data
    (if (and (== (Utilities|Array|Length (.HandKeyLocations (Utilities|Struct|BreakXRHandTrackingState _handtrackingstate))) 26) (== (Utilities|Array|Length (.HandKeyRotations (Utilities|Struct|BreakXRHandTrackingState _handtrackingstate))) 26))
      ;[0.0156 0.15 0.008148 0.5] create a Joint Transform from the fetched loc-rot data
      (for (_ _array_index) (.HandKeyLocations (Utilities|Struct|BreakXRHandTrackingState _handtrackingstate))
        (Utilities|Array|Add (LocalVariables|GetJoint%20Transforms) (Math|Transform|MakeTransform (Utilities|Array|Get(acopy) (.HandKeyLocations (Utilities|Struct|BreakXRHandTrackingState _handtrackingstate)) _array_index) (Class|KismetMathLibrary|QuatRotator (Utilities|Array|Get(acopy) (.HandKeyRotations (Utilities|Struct|BreakXRHandTrackingState _handtrackingstate)) _array_index)) "0.010000,0.010000,0.010000")))
      ;[0.07111 0.8802 0 0.5] after loop, return that created Joint Transform obj
      (return (LocalVariables|GetJoint%20Transforms))
      (else
        _)))
  ;[0.15 0 0 0.5] if the hand data doesnt validate, return no (empty) transform
  (return 0))

(fn ClearHands
  (Components|InstancedStaticMesh|ClearInstances (Variables|Components|GetInstancedStaticMesh)))

(fn DrawHand
  (params (Joint%20Transforms :type Array%20of%20Transforms))
  (for _array_element Joint%20Transforms
    (Components|InstancedStaticMesh|AddInstance (Variables|Components|GetInstancedStaticMesh) _array_element true)))

(fn CheckGestures
  (params (Joint%20Transforms :type Array%20of%20Transforms))
  (bind _isvalidjointtransform (CallFunction|IsJointTransformValid Joint%20Transforms))
  (if _isvalidjointtransform
    ;[0.15 0.15 0.15 0.5] Check if we are starting or ending a spell chain
    (bind _posture_met (CallFunction|Handpose:Gun Joint%20Transforms))
    (if _posture_met
      (goto _label Break)
      (else
        (bind _posture_met_2 (CallFunction|Handpose:SipsTea Joint%20Transforms))
        (if _posture_met_2
          (Utilities|Array|Clear (Variables|Default|GetSpell%20Feed))
          (Utilities|FlowControl|ForLoopwithBreak 0 10 :!label _label
            (:LoopBody
              ;[0.15 0.15 0.15 0.5] Loop body: transcribe spell postures
              (bind _posture (CallFunction|ReadPosture Joint%20Transforms))
              (Variables|Default|SetCurrent%20Posture _posture)
              (CallFunction|ReadPosture))))))))

(fn IsJointTransformValid
  (params (Joint%20Transforms :type Array%20of%20Transforms))
  (return (== (Utilities|Array|Length Joint%20Transforms) 26)))

(fn ReadPosture
  (params (Joint%20Transform :type Array%20of%20Transforms))
  ;[0.15 0.15 0.15 0.5] Base Elements
  (bind _posture_met (CallFunction|Handpose:Flat Joint%20Transform))
  (if _posture_met
    ;[1 1 1 0.5] Air
    (bind _posture_met_2 (CallFunction|HandFacingUp Joint%20Transform))
    (if _posture_met_2
      (CallFunction|ChangeHandMaterial "/Game/Handcasting/Materials/HandCubes_Casting_Air.HandCubes_Casting_Air")
      (return "Air")
      (else
        ;[1 0.1057 0 0.5] Fire
        (bind _posture_met_3 (CallFunction|HandFacingLeft Joint%20Transform))
        (if _posture_met_3
          (CallFunction|ChangeHandMaterial "/Game/Handcasting/Materials/HandCubes_Casting_Fire.HandCubes_Casting_Fire")
          (return "Fire")
          (else
            ;[0 0.06912 0.901 0.5] Water
            (bind _posture_met_4 (CallFunction|HandFacingRight Joint%20Transform))
            (if _posture_met_4
              (CallFunction|ChangeHandMaterial "/Game/Handcasting/Materials/HandCubes_Casting_Water.HandCubes_Casting_Water")
              (return "Water")
              (else
                ;[0.02966 0.2656 0.02536 0.5] Earth
                (bind _posture_met_5 (CallFunction|HandFacingDown Joint%20Transform))
                (if _posture_met_5
                  (CallFunction|ChangeHandMaterial "/Game/Handcasting/Materials/HandCubes_Casting_Earth.HandCubes_Casting_Earth")
                  (return "Earth")
                  (else
                    _))))))))
    (else
      ;[0.15 0.15 0.15 0.5] Shape: Projectile
      (bind _posture_met_6 (CallFunction|Handpose:Gun Joint%20Transform))
      (if _posture_met_6
        (CallFunction|ChangeHandMaterial "/Game/Handcasting/Materials/HandCubes_Casting_Projectile.HandCubes_Casting_Projectile")
        (return "Projectile")
        (else
          ;[0.15 0.15 0.15 0.5] Shape: Special
          (bind _posture_met_7 (CallFunction|Handpose:Claw Joint%20Transform))
          (if _posture_met_7
            (CallFunction|ChangeHandMaterial "/Game/Handcasting/Materials/HandCubes_Casting_Projectile.HandCubes_Casting_Projectile")
            (return "Special")
            (else
              _))))))
  (return "None"))

(fn ChangeHandMaterial
  (params (Material :type Material%20Object%20Reference))
  (Rendering|Material|SetMaterial (Variables|Components|GetInstancedStaticMesh) 0 Material))

(fn CastSpell
  (params (Joint%20Transform :type Array%20of%20Transforms) (Spell%20Name :type Name))
  (bind _returnvalue (Utilities|Enum|LiteralenumEHandKeypoint "IndexMetacarpal"))
  (bind _returnvalue_2 (Utilities|Enum|LiteralenumEHandKeypoint "Palm"))
  (bind _returnvalue_3 (Class|HandKeypointConversion|ToInt32(HandKeypoint) _returnvalue_2))
  (bind _returnvalue_4 (Class|HandKeypointConversion|ToInt32(HandKeypoint) _returnvalue))
  (bind _output (Utilities|Array|Get(acopy) Joint%20Transform _returnvalue_4))
  (bind _output_2 (Utilities|Array|Get(acopy) Joint%20Transform _returnvalue_3))
  (bind _returnvalue_5 (Math|Vector|GetForwardVector (.rotation _output_2)))
  (bind _returnvalue_6 (Math|Conversions|RotationFromXVector _returnvalue_5))
  (bind _returnvalue_7 (Math|Transform|MakeTransform (.location _output) _returnvalue_6))
  (if (== Spell%20Name "Fire Bolt")
    (CallFunction|FireProjectile _returnvalue_7)
    (elif (== Spell%20Name "Ice Bolt")
      (CallFunction|WaterProjectile _returnvalue_7)
      (elif (== Spell%20Name "Air Bolt")
        (CallFunction|AirProjectile _returnvalue_7)
        (elif (== Spell%20Name "Earth Bolt")
          (CallFunction|EarthProjectile _returnvalue_7)
          (elif (== Spell%20Name "Earth Pillar")
            (bind _raycast_location (CallFunction|ComputeRaycastLocation Joint%20Transform))
            (CallFunction|EarthPillar _raycast_location)
            (elif (== Spell%20Name "Scorch")
              (bind _raycast_location_2 (CallFunction|ComputeRaycastLocation Joint%20Transform))
              (CallFunction|Scorch _raycast_location_2))))))))